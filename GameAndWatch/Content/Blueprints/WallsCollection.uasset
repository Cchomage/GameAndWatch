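; WallsCollection spawns and holds a set of Walls actors when play begins, one for each slot in WallArray.
; Each spawned wall is stored back into the array and takes its Paper2D sprite from SpriteArray at the same index.
; All sprites share one fixed world transform, while each wall's Cube takes location and rotation from the parallel TransformArray with a fixed, thinned scale.
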(event EventBeginPlay
  (for (_ _array_index) (Variables|Default|GetWallArray)
    (bind _returnvalue (Game|SpawnActorfromClass "/Game/Blueprints/Walls.Walls_C" (Math|Transform|MakeTransform "0, 0, 0" "0, 0, 0" "1,1,1") "Undefined" 0 0))
    (Utilities|Array|SetArrayElem (Variables|Default|GetWallArray) _array_index _returnvalue)
    (Rendering|Components|Sprite|SetSprite (Variables|/Game/Blueprints/Walls.Walls_C|GetPaperSprite _returnvalue) (Utilities|Array|Get(acopy) (Variables|Default|GetSpriteArray) _array_index))
    (Transformation|SetWorldTransform (Variables|/Game/Blueprints/Walls.Walls_C|GetPaperSprite _returnvalue) (Math|Transform|MakeTransform "130.000000,80.000000, 0" "0,90.000000,-90.000000" "0.200000,1,0.200000") false false)
    (Transformation|SetWorldTransform (Variables|/Game/Blueprints/Walls.Walls_C|GetCube _returnvalue) (Math|Transform|MakeTransform (.location (Utilities|Array|Get(acopy) (Variables|Default|GetTransformArray) _array_index)) (.rotation (Utilities|Array|Get(acopy) (Variables|Default|GetTransformArray) _array_index)) "1.000000,0.200000,1.000000") false false)))

(fn ConstructionScript)