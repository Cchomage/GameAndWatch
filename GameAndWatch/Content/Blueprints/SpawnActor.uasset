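; Enemy spawner actor that spawns EnemyAi at random intervals, which tend to shorten as play time passes.
; Chained Delay nodes on Tick act as repeating timers: the first accumulates Timing, the second waits a random time whose upper bound shrinks with Timing, unclamped.
; Each spawn prints a debug string and places the enemy just ahead of the root component, matching its rotation and ignoring collisions.
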(event Custom|Spawn)

(event Custom|Diff2)

(event EventBeginPlay)

(event EventTick
  (params (DeltaSeconds :type Float%20%28single-precision%29))
  (bind _defaultsceneroot (Variables|Default|GetDefaultSceneRoot))
  (Utilities|FlowControl|Delay 0.5)
  (Variables|Default|SetTiming (+ (Variables|Default|GetTiming) 0.5))
  (Utilities|FlowControl|Delay (Math|Random|RandomFloatinRange 5.0 (- 3e+01 (/ (Variables|Default|GetTiming) 15.0))))
  (Development|PrintString "Hello")
  (Game|SpawnActorfromClass "/Game/Blueprints/EnemyAi.EnemyAi_C" (Math|Transform|MakeTransform (+ (Transformation|GetWorldLocation _defaultsceneroot) (* (Math|Vector|GetForwardVector _defaultsceneroot) 50)) (Transformation|GetWorldRotation _defaultsceneroot)) "AlwaysSpawn" 0 0))

(fn ConstructionScript)