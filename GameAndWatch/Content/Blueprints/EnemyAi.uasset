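; Enemy actor that advances along EnemyPath tiles, destroys itself with any wall it meets, and triggers a game loss otherwise.
; A looping timer line-traces ahead of its Box each second and teleports it onto the detected tile at fixed height.
; When the trace hits a CharacterPAth, a shorter trace ignoring that actor finds the tile.
; Any other result, including no hit, sets GameLoss, destroys the enemy and reloads ThirdPersonExampleMap.
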(event Custom|RestartGame
  (Game|OpenLevel(byObjectReference) "/Game/Blueprints/Maps/ThirdPersonExampleMap.ThirdPersonExampleMap"))

(event Custom|LineTraceAi
  (bind _box (Variables|Default|GetBox))
  (bind _box_2 (Variables|Default|GetBox))
  (bind _returnvalue (Transformation|GetWorldLocation _box_2))
  (bind _returnvalue_2 (Math|Vector|GetForwardVector _box_2))
  (bind _returnvalue_3 (Transformation|GetWorldLocation _box))
  (bind _returnvalue_4 (Math|Vector|GetForwardVector _box))
  (bind _outhit (Collision|LineTraceByChannel (+ _returnvalue (* _returnvalue_2 50)) (+ _returnvalue (* _returnvalue_2 400)) "TraceTypeQuery1" false 0 "None"))
  (bind _ascharacter_path (Utilities|Casting|CastToCharacterPAth (.hitactor _outhit))
    (:then
      (bind _outhit_2 (Collision|LineTraceByChannel (+ _returnvalue_3 (* _returnvalue_4 50)) (+ _returnvalue_3 (* _returnvalue_4 200)) "TraceTypeQuery1" false (Utilities|Array|MakeArray _ascharacter_path) "None"))
      (bind _asenemy_path (Utilities|Casting|CastToEnemyPath (.hitactor _outhit_2)))
      (Transformation|SetWorldLocation (Variables|Default|GetBox) (Math|Vector|MakeVector (.X (Math|Vector|BreakVector (Transformation|GetWorldLocation (Variables|/Game/Blueprints/Path/EnemyPath.EnemyPath_C|GetBox _asenemy_path)))) (.Y (Math|Vector|BreakVector (Transformation|GetWorldLocation (Variables|/Game/Blueprints/Path/EnemyPath.EnemyPath_C|GetBox _asenemy_path)))) 2e+01) false true))
    (:CastFailed
      (bind _asenemy_path_2 (Utilities|Casting|CastToEnemyPath (.hitactor _outhit))
        (:then
          (Transformation|SetWorldLocation (Variables|Default|GetBox) (Math|Vector|MakeVector (.X (Math|Vector|BreakVector (Transformation|GetWorldLocation (Variables|/Game/Blueprints/Path/EnemyPath.EnemyPath_C|GetBox _asenemy_path_2)))) (.Y (Math|Vector|BreakVector (Transformation|GetWorldLocation (Variables|/Game/Blueprints/Path/EnemyPath.EnemyPath_C|GetBox _asenemy_path_2)))) 2e+01) false true))
        (:CastFailed
          (bind _aswalls (Utilities|Casting|CastToWalls (.hitactor _outhit))
            (:then
              (Utilities|IsValid "/Game/Blueprints/Walls.Walls"
                (:Is%20Valid
                  (Actor|DestroyActor _aswalls)
                  (Utilities|IsValid self
                    (:Is%20Valid
                      (Actor|DestroyActor))))))
            (:CastFailed
              (Development|PrintString "YOU LOOSE")
              (Variables|Default|SetGameLoss true)
              (Actor|DestroyActor)
              (CallFunction|RestartGame))))))))

(event EventBeginPlay
  ;[1 1 1] MovementSpeed(Timing=Rate at which movement ticks)
  (Utilities|Time|SetTimerbyEvent (delegate Custom|LineTraceAi) 1.0 true))

(fn ConstructionScript)